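; Director actor for a cover-point demo that drives cover agents, a threat and a cover volume.
; On BeginPlay it caches the agents, registers the threat, stores a cover volume and enables debug draw.
; Its events cycle the threat through four fixed positions and re-request cover, deploy agents, rebuild the cover field, release all claims or toggle debug draw.
; Most actions update a status string.
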(event Custom|DeployAgents
  (for _array_element (Variables|Default|GetAgents)
    (bind _asbp_cover_agent (Utilities|Casting|CastToBP_CoverAgent _array_element))
    (Default|RequestCover _asbp_cover_agent))
  (Variables|Default|SetStatus "Agents deployed"))

(event Custom|BuildCoverField
  (Class|CoverPointsStatics|RebuildVolume (Variables|Default|GetVolume))
  (Class|CoverPointsStatics|SetShowCoverPoints true)
  (Class|CoverPointsStatics|SetShowPeekSides true)
  (Variables|Default|SetShowDebug true)
  (Variables|Default|SetStatus "Building cover field"))

(event Custom|ReleaseAllClaims
  (for _array_element (Variables|Default|GetAgents)
    (bind _asbp_cover_agent (Utilities|Casting|CastToBP_CoverAgent _array_element))
    (Default|ReleaseandReset _asbp_cover_agent))
  (Class|CoverPointsStatics|ReleaseAllCover)
  (Variables|Default|SetStatus "All claims released"))

(event Custom|ToggleDebugDraw
  (bind _returnvalue (Class|CoverPointsStatics|IsShowingCoverPoints))
  (bind _returnvalue_2 (not _returnvalue))
  (Class|CoverPointsStatics|SetShowCoverPoints _returnvalue_2)
  (Class|CoverPointsStatics|SetShowPeekSides _returnvalue_2)
  (Variables|Default|SetShowDebug _returnvalue_2))

(event Custom|AdvanceThreat
  (if (> (+ (Variables|Default|GetThreatIndex) (Class|KismetSystemLibrary|MakeLiteralInteger 1)) (Class|KismetSystemLibrary|MakeLiteralInteger 3))
    (Variables|Default|SetThreatIndex 0)
    (else
      (Variables|Default|SetThreatIndex (+ (Variables|Default|GetThreatIndex) (Class|KismetSystemLibrary|MakeLiteralInteger 1)))))
  (if (== (Variables|Default|GetThreatIndex) (Class|KismetSystemLibrary|MakeLiteralInteger))
    (Variables|Default|SetThreatTarget (Math|Vector|MakeVector 2.4e+03 0.0 -8.0))
    (elif (== (Variables|Default|GetThreatIndex) (Class|KismetSystemLibrary|MakeLiteralInteger 1))
      (Variables|Default|SetThreatTarget (Math|Vector|MakeVector 0.0 2.4e+03 -8.0))
      (elif (== (Variables|Default|GetThreatIndex) (Class|KismetSystemLibrary|MakeLiteralInteger 2))
        (Variables|Default|SetThreatTarget (Math|Vector|MakeVector -2.4e+03 4e+02 -8.0))
        (else
          (Variables|Default|SetThreatTarget (Math|Vector|MakeVector 3e+02 -2.4e+03 -8.0))))))
  (Transformation|SetActorLocation (Variables|Default|GetThreat) (Variables|Default|GetThreatTarget) false false)
  (for _array_element (Variables|Default|GetAgents)
    (bind _asbp_cover_agent (Utilities|Casting|CastToBP_CoverAgent _array_element))
    (Default|RequestCover _asbp_cover_agent))
  (Variables|Default|SetStatus "Threat moved - agents redeployed"))

(event EventBeginPlay
  (bind _outactors (Actor|GetAllActorsOfClass "/CoverPoints/CoverPoints/Blueprints/BP_CoverAgent.BP_CoverAgent_C"))
  (Variables|Default|SetAgents _outactors)
  (bind _outactors_2 (Actor|GetAllActorsOfClass "/CoverPoints/CoverPoints/Blueprints/BP_CoverThreat.BP_CoverThreat_C"))
  (for _array_element _outactors_2
    (Variables|Default|SetThreat _array_element)
    (Class|CoverPointsStatics|SetThreatActor _array_element))
  (for _array_element_2 (Class|CoverPointsStatics|GetAllCoverVolumes)
    (Variables|Default|SetVolume _array_element_2))
  (Variables|Default|SetThreatIndex 0)
  (Class|CoverPointsStatics|SetShowCoverPoints true)
  (Class|CoverPointsStatics|SetShowPeekSides true)
  (Variables|Default|SetShowDebug true)
  (Variables|Default|SetStatus "Ready"))

(fn ConstructionScript)