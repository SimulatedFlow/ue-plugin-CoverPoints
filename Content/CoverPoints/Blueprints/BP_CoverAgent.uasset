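; BP_CoverAgent is an agent actor that moves into cover from a threat and back home on request.
; RequestCover queries FindBestCover around the threat, storing the target point and a peek-side label, or flagging no cover.
; ReleaseAndReset frees its cover and retargets the spawn location.
; Tick interpolates straight to the target without navigation or sweep, facing the threat.
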(event Custom|RequestCover
  (bind _returnvalue (Class|CoverPointsStatics|FindBestCover self (Class|CoverPointsStatics|GetThreatLocation) 9e+03 true "(ShieldingWeight=3.000000,AgentDistanceWeight=1.000000,ThreatDistanceWeight=1.000000,HighCoverWeight=0.750000,PeekWeight=1.000000,WallProximityWeight=0.500000,PreferredThreatDistance=1200.000000,MinShielding=0.300000,bRequireHighCover=False,bRequirePeek=False,bAllowClaimed=False)"))
  (if (.bFound (Utilities|Struct|BreakCoverQueryResult _returnvalue))
    (Variables|Default|SetCoverTarget (.Location (Utilities|Struct|BreakCoverPoint (.Point (Utilities|Struct|BreakCoverQueryResult _returnvalue)))))
    (Variables|Default|SetHasCover true)
    (Variables|Default|SetPeekLabel (Class|CoverPointsStatics|PeekSidetoString (.PeekSide (Utilities|Struct|BreakCoverQueryResult _returnvalue))))
    (else
      (Variables|Default|SetHasCover false)
      (Variables|Default|SetPeekLabel "no cover"))))

(event Custom|ReleaseAndReset
  (Class|CoverPointsStatics|ReleaseCoverforActor self)
  (Variables|Default|SetHasCover false)
  (Variables|Default|SetPeekLabel "-")
  (Variables|Default|SetCoverTarget (Variables|Default|GetHomeLocation)))

(event EventBeginPlay
  (bind _self self)
  (bind _returnvalue (Transformation|GetActorLocation _self))
  (Variables|Default|SetHomeLocation _returnvalue)
  (Variables|Default|SetCoverTarget _returnvalue)
  (Variables|Default|SetPeekLabel "-"))

(event EventTick
  (params (DeltaSeconds :type Float%20%28single-precision%29))
  (bind _self self)
  (bind _covertarget (Variables|Default|GetCoverTarget))
  (bind _movespeed (Variables|Default|GetMoveSpeed))
  (bind _returnvalue (Transformation|GetActorLocation _self))
  (bind _returnvalue_2 (Math|Interpolation|VInterpTo _returnvalue _covertarget DeltaSeconds _movespeed))
  (Transformation|SetActorLocation _self _returnvalue_2 false false)
  (Transformation|SetActorRotation _self (Math|Rotator|FindLookatRotation _returnvalue_2 (Class|CoverPointsStatics|GetThreatLocation))))

(fn ConstructionScript)